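; Player controller for DomeKeeper that holds the resource inventory and bought items behind a skill tree.
; Left click opens the skill tree widget in UI-only input, and E adds one resource and refreshes its colors.
; Purchase checks require unowned items, owned parents resolved through DT_DK_Item, and enough resources.
; RemoveRessources records the bought item and deducts its costs from the inventory map.
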(event `Key|LeftMouseButton`
  (params (Key :type "Key Structure"))
  (:`Pressed`
    (bind _returnvalue (`|CreateWidget` "/Game/DomeKeeper/Widget/WBP_SkillTree.WBP_SkillTree_C"))
    (set `self.SkillTree` _returnvalue)
    (`WidgetBlueprintLibrary.SetInputMode_UIOnlyEx` self (`self.SkillTree`) "DoNotLock" true)
    (`UserWidget.AddToViewport` (`self.SkillTree`) 0)
    (`Widget.SetUserFocus` (`self.SkillTree`) self)))

(event `Key|E`
  (params (Key :type "Key Structure"))
  (bind _inventory (`self.Inventory`))
  (:`Pressed`
    (`BlueprintMapLibrary.Map_Add` _inventory "NewEnumerator1" (+ (`BlueprintMapLibrary.Map_Find` _inventory "NewEnumerator1") 1))
    (bind _skilltree (`self.SkillTree`)
      (:`then`
        (`/Game/DomeKeeper/Widget/WBP_SkillTree.RefreshSetColor` _skilltree))
      (:`else`))))

(event `RemoveRessources`
  (bind _inventory (`self.Inventory`))
  (`KismetArrayLibrary.Array_Add` (`self.Items`) (`self.Item to Buy`))
  (bind _keys (`BlueprintMapLibrary.Map_Keys` (`.NeedRessources_50_C1264C7E467D7C023665B0A7AC81A21C` (break `/Game/DomeKeeper/S_DK_Item` (`self.Item to Buy`)))))
  (for _array_element _keys
    (`BlueprintMapLibrary.Map_Add` _inventory _array_element (+ (`BlueprintMapLibrary.Map_Find` _inventory _array_element) (* (`BlueprintMapLibrary.Map_Find` (`.NeedRessources_50_C1264C7E467D7C023665B0A7AC81A21C` (break `/Game/DomeKeeper/S_DK_Item` (`self.Item to Buy`))) _array_element) -1)))))

(fn `UserConstructionScript`)

(fn `VerificationCanBuy`
  (params (ItemToBuy :type "/Game/DomeKeeper/S_DK_Item Structure (by ref)"))
  (returns (Return :type Boolean))
  (locals (`CanBuy?` :type Boolean :default true))
  (set `self.Item to Buy` ItemToBuy)
  (bind _haveitem_ (`self.VerificationHaveItems`))
  (if (or (not _haveitem_) (`KismetArrayLibrary.Array_Contains` (`self.Items`) (`self.Item to Buy`)))
    (return false)
    (else
      (set `local.CanBuy?` true)
      (bind _keys (`BlueprintMapLibrary.Map_Keys` (`.NeedRessources_50_C1264C7E467D7C023665B0A7AC81A21C` (break `/Game/DomeKeeper/S_DK_Item` (`self.Item to Buy`)))))
      (for _array_element _keys
        (if (< (- (`BlueprintMapLibrary.Map_Find` (`self.Inventory`) _array_element) (`BlueprintMapLibrary.Map_Find` (`.NeedRessources_50_C1264C7E467D7C023665B0A7AC81A21C` (break `/Game/DomeKeeper/S_DK_Item` (`self.Item to Buy`))) _array_element)) 0)
          (set `local.CanBuy?` false)
          (break)))
      (return (`local.CanBuy?`)))))

(fn `VerificationHaveItems`
  (returns (`HaveItem?` :type Boolean))
  (locals (`GetPreviousItem?` :type Boolean :default true))
  (set `local.GetPreviousItem?` true)
  (for _array_element (`.ParentsItems_55_78A45E8943A2FB9CD0F4DDBDD52CA03E` (break `/Game/DomeKeeper/S_DK_Item` (`self.Item to Buy`)))
    (bind _returnvalue (`|GetDataTableRow` "/Game/DomeKeeper/DT_DK_Item.DT_DK_Item" (`KismetStringLibrary.Conv_StringToName` (`|GetEnumeratorNameAsString` _array_element)))
      (:`then`
        (if (not (`KismetArrayLibrary.Array_Contains` (`self.Items`) _returnvalue))
          (set `local.GetPreviousItem?` false)
          (break)))
      (:`RowNotFound`
        (`KismetSystemLibrary.PrintString` "Error")
        (break))))
  (return (`local.GetPreviousItem?`)))