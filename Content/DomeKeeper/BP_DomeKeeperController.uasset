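; Player controller for DomeKeeper that holds a resource Inventory map and opens the skill tree UI.
; Left click creates a new WBP_SkillTree, adds it to the viewport and sets user focus on it.
; E increments one resource and calls a custom event on the skill tree.
; RemoveRessources loops over the passed map's keys, subtracting each key's loop index, not its mapped amount, from the Inventory.
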(event `Key|LeftMouseButton`
  (params (Key :type "Key Structure"))
  (:`Pressed`
    (bind _returnvalue (`|CreateWidget` "/Game/DomeKeeper/Widget/WBP_SkillTree.WBP_SkillTree_C"))
    (set `self.SkillTree` _returnvalue)
    (`UserWidget.AddToViewport` (`self.SkillTree`) 0)
    (`Widget.SetUserFocus` (`self.SkillTree`) self)))

(event `Key|E`
  (params (Key :type "Key Structure"))
  (bind _inventory (`self.Inventory`))
  (:`Pressed`
    (`BlueprintMapLibrary.Map_Add` _inventory "NewEnumerator1" (+ (`BlueprintMapLibrary.Map_Find` _inventory "NewEnumerator1") 1))
    (bind _skilltree (`self.SkillTree`)
      (:`then`
        (`/Game/DomeKeeper/Widget/WBP_SkillTree.CustomEvent` _skilltree))
      (:`else`))))

(event `RemoveRessources`
  (params (RessourcesToRemove :type "Map of /Game/DomeKeeper/Enum/E_DK_Ressources Enum to Integer"))
  (bind _inventory (`self.Inventory`))
  (set `self.Ressources to Remove` RessourcesToRemove)
  (bind _keys (`BlueprintMapLibrary.Map_Keys` (`self.Ressources to Remove`)))
  (for (_array_element _array_index) _keys
    (`BlueprintMapLibrary.Map_Add` _inventory _array_element (+ (`BlueprintMapLibrary.Map_Find` _inventory _array_element) (* _array_index -1)))))

(fn `UserConstructionScript`)