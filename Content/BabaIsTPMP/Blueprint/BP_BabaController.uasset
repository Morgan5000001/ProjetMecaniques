(event `self.ReceiveBeginPlay`
  ;[1 1 1] BeginPlay
  (`EnhancedInputSubsystemInterface.AddMappingContext` (pcsubsystem `EnhancedInputLocalPlayerSubsystem` (`GameplayStatics.GetPlayerController` 0)) "/Game/ThirdPerson/Input/IMC_Default.IMC_Default" 0 (struct)))

(event `Key|M`
  (params (Key :type "Key Structure"))
  ;[0 0 0] Debug pour Dev
  (:`Pressed`
    (`/Engine/EditorBlueprintResources/StandardMacros.FlipFlop`
      (:`A`
        (set `self.DebugTraceDeplacement` "ForDuration"))
      (:`B`
        (set `self.DebugTraceDeplacement` "None")))))

(event `EnhancedInput|/Game/ThirdPerson/Input/Actions/IA_Move`
  (params (ActionValue :type "Vector2D Structure") (ElapsedSeconds :type "Float (double-precision)") (TriggeredSeconds :type "Float (double-precision)") (InputAction :type "InputAction Object Reference" :default "/Game/ThirdPerson/Input/Actions/IA_Move.IA_Move"))
  (bind _timedeplacement (`self.TimeDeplacement`))
  (:`Started`
    (bind _returnvalue (`KismetSystemLibrary.K2_SetTimerDelegate` (delegate `Deplacement`) _timedeplacement true (* _timedeplacement -1.0)))
    (set `self.TimerDeplacement` _returnvalue))
  (:`Completed`
    (`KismetSystemLibrary.K2_ClearAndInvalidateTimerHandle` (`self.TimerDeplacement`))))

(event `Deplacement`
  (bind (_returnvalue_x _returnvalue_y) (`KismetMathLibrary.BreakVector2D` (`|GetInputActionValue`)))
  (bind (_returnvalue_x_2 _returnvalue_y_2) (`KismetMathLibrary.BreakVector2D` (`|GetInputActionValue`)))
  (bind (_returnvalue_x_3 _returnvalue_y_3) (`KismetMathLibrary.BreakVector2D` (`|GetInputActionValue`)))
  (bind _returnvalue (`KismetMathLibrary.Vector_SnappedToGrid` (+ (`self.K2_GetActorLocation` (`self.K2_GetPawn`)) (`KismetMathLibrary.MakeVector` (* _returnvalue_y_3 120.0) (* _returnvalue_x_3 120.0))) 120.0))
  (if (not (and (== (`KismetMathLibrary.Abs` _returnvalue_x) 1.0) (== (`KismetMathLibrary.Abs` _returnvalue_y) 1.0)))
    (bind (_outhit _returnvalue_2) (`KismetSystemLibrary.LineTraceSingle` :`Start` _returnvalue :`End` (- _returnvalue (0.0 0.0 150.0)) :`TraceChannel` "TraceTypeQuery1" :`DrawDebugType` (`self.DebugTraceDeplacement`)))
    (bind (_bblockinghit _binitialoverlap _time _distance _location _impactpoint _normal _impactnormal _physmat _hitactor) (`GameplayStatics.BreakHitResult` _outhit))
    (if (`KismetSystemLibrary.DoesImplementInterface` _hitactor "/Game/BabaIsTPMP/Blueprint/BPI_BabaInteract.BPI_BabaInteract_C")
      (message `/Game/BabaIsTPMP/Blueprint/BPI_BabaInteract.Pousser` _hitactor (`KismetMathLibrary.MakeVector` (* _returnvalue_y_2 120.0) (* _returnvalue_x_2 120.0)))
      (`self.K2_SetActorLocation` (`self.K2_GetPawn`) (`KismetMathLibrary.MakeVector` (.x _returnvalue) (.y _returnvalue) 120.0) false false :!label _label)
      (elif _returnvalue_2
        (goto _label)))))

(fn `UserConstructionScript`)