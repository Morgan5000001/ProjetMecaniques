(event `self.ReceiveBeginPlay`
  (bind (_returnvalue_x _returnvalue_y) (`KismetMathLibrary.BreakVector` (`KismetMathLibrary.Vector_SnappedToGrid` (`self.K2_GetActorLocation`) 120.0)))
  (`self.K2_SetActorLocation` (`KismetMathLibrary.MakeVector` _returnvalue_x _returnvalue_y 50.0))
  ;[1 1 1] Get all actor of class maison
  (switch `/Game/BabaIsTPMP/Blueprint/EN_BabaType` (`self.Type`)
    (:`NewEnumerator1`
      (bind _asbp_baba_controller (cast `/Game/BabaIsTPMP/Blueprint/BP_BabaController` (`GameplayStatics.GetPlayerController` 0)))
      (`KismetArrayLibrary.Array_Add` (`/Game/BabaIsTPMP/Blueprint/BP_BabaController.PossesActors` _asbp_baba_controller) self))))

(fn `Pousser`
  (params (Direction :type "Vector Structure"))
  (returns (`ShouldMove?` :type Boolean))
  (locals (NextLocation :type "Vector Structure" :default (0.0 0.0 0.0)))
  (if (not (`|EnumEquality` (`self.Type`) "NewEnumerator3"))
    (bind _output_get (set `local.NextLocation` (`KismetMathLibrary.Vector_SnappedToGrid` (+ Direction (`self.K2_GetActorLocation`) (0.0 0.0 50.0)) 120.0)))
    (bind (_outhit _returnvalue) (`KismetSystemLibrary.LineTraceSingle` _output_get (- _output_get (0.0 0.0 150.0)) "TraceTypeQuery1"))
    (if _returnvalue
      (bind (_bblockinghit _binitialoverlap _time _distance _location _impactpoint _normal _impactnormal _physmat _hitactor) (`GameplayStatics.BreakHitResult` _outhit))
      (if (`KismetSystemLibrary.DoesImplementInterface` _hitactor "/Game/BabaIsTPMP/Blueprint/BPI_BabaInteract.BPI_BabaInteract_C")
        (bind _shouldmove_ (message `/Game/BabaIsTPMP/Blueprint/BPI_BabaInteract.Pousser` _hitactor Direction))
        (if _shouldmove_
          (`self.K2_SetActorLocation` (`KismetMathLibrary.MakeVector` (.x (`local.NextLocation`)) (.y (`local.NextLocation`)) 50.0))
          (return true) ; Le bloc d'après se décale, donc on peut toout décaler
          (else
            (return false) ; Le bloc d'après ne peut pas se décaler dans le sens, donc on pousse rien
          ))
        (else
          (`self.K2_SetActorLocation` (`KismetMathLibrary.MakeVector` (.x (`local.NextLocation`)) (.y (`local.NextLocation`)) 50.0))
          (return true) ; On peut pas pousser l'objet d'après donc on peut y aller
        ))
      (else
        (return false) ; On a rien hit après, donc il y a du vide, donc ne pousse pas
      ))
    (else
      (return false) ; On peut pas te bouger
    )))

(fn `UserConstructionScript`
  (bind _cube (`self.Cube`))
  (switch `/Game/BabaIsTPMP/Blueprint/EN_BabaType` (`self.Type`)
    (:`NewEnumerator1`
      (`PrimitiveComponent.SetMaterial` _cube 0 "/Game/BabaIsTPMP/Material/MI_BabaPlayer.MI_BabaPlayer"))
    (:`NewEnumerator2`
      (`PrimitiveComponent.SetMaterial` _cube 0 "/Game/BabaIsTPMP/Material/MI_BabaPush.MI_BabaPush"))
    (:`NewEnumerator3`
      (`PrimitiveComponent.SetMaterial` _cube 0 "/Game/BabaIsTPMP/Material/MI_BabaWall.MI_BabaWall"))))